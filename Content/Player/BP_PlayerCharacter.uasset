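; Player vehicle for an arcade score game, driven by forces on a physics cube, with drift effects, speed-based camera and ram damage.
; Combo points bank into Score when their timer expires; staying too slow drains FailTimer, which saves the high score and shows the fail screen.
; Weighted DataTable picks fill upgrade choice screens; physical upgrades attach as actors or level up existing ones.
; Tunable stats live in an enum-indexed Properties array.
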(event Custom|RequestUpgrade
  ;[0.07812 1 0] Request Upgrade cards
  (bind _returnvalue (UserInterface|CreateWidget "/Game/Upgrades/Base/UI_UpgradeChooseScreen.UI_UpgradeChooseScreen_C" 0 (Utilities|Array|MakeArray (CallFunction|GetRandomUpgrade) (CallFunction|GetRandomUpgrade) (CallFunction|GetRandomUpgrade))))
  (UserInterface|Viewport|AddtoViewport _returnvalue 0))

(event Custom|AddScoreEvent
  (params (Amount :type Integer) (Reason :type E_PointScoreReason%20Enum :default "NewEnumerator0"))
  ;[0 1 1] Add Score
  (Variables|Default|SetCurrentCombo (+ (Variables|Default|GetCurrentCombo) Amount))
  (Utilities|FlowControl|Sequence
    (:then_0
      (if (Utilities|Enum|NotEqual(Enum) Reason "NewEnumerator1")
        (Variables|Default|SetComboTime 5.0)))
    (:then_1
      (Default|CallAddScore)
      (Variables|Default|SetLastScoreReason Reason)
      (Utilities|FlowControl|DoOnce false
        (:Completed
          (bind _returnvalue (Utilities|Time|SetTimerbyEvent (delegate Custom|AddComboScore) 1e+01 true))
          (Variables|Default|SetComboTimer _returnvalue))))))

(event Custom|AddComboScore
  ;[0 1 1] Add Score
  (CallFunction|AddScoreEvent 5 "NewEnumerator1"))

(event Custom|ResetComboScoreTimer
  ;[0 1 1] Add Score
  (Utilities|Time|ClearandInvalidateTimerbyHandle (Variables|Default|GetComboTimer))
  (Utilities|FlowControl|DoOnce false) ; enters at Reset
)

(event EventBeginPlay
  (bind _returnvalue (Game|GetPlayerController 0))
  (bind _asbp_player_controller (Utilities|Casting|CastToBP_PlayerController (Game|GetPlayerController 0)))
  (Input|AddMappingContext (PlayerController|LocalPlayerSubsystems|GetEnhancedInputLocalPlayerSubsystem _asbp_player_controller) "/Game/Player/Input/IMC_Inputs.IMC_Inputs" 0 "(bIgnoreAllPressedKeysUntilRelease=True,bForceImmediately=False)")
  (CallFunction|ResetProperties)
  (bind _returnvalue_2 (UserInterface|CreateWidget "/Game/Player/Widgets/UI_HUD.UI_HUD_C"))
  (bind _output_get (Variables|Default|SetUI _returnvalue_2))
  (UserInterface|Viewport|AddtoViewport _output_get 0)
  (Input|SetInputModeGameOnly _returnvalue true)
  (Variables|/Script/Engine.PlayerController|SetbShowMouseCursor _returnvalue false)
  (bind _returnvalue_3 (Utilities|Time|SetTimerbyEvent (EventDispatchers|CreateEvent :!event Custom|RequestUpgrade) 3e+01 true))
  (Variables|Default|SetUpgradeTimer _returnvalue_3)
  ;[1 0.1641 0] UpgradeWeights
  (bind _outrownames (DataTable|GetDataTableRowNames "/Game/Upgrades/DT_Upgrades.DT_Upgrades"))
  (Variables|Default|SetUpgradeRowNames _outrownames)
  (bind _returnvalue_4 (|GetDataTableasArrayStruct "/Game/Upgrades/DT_Upgrades.DT_Upgrades"))
  (for (_array_element _array_index) _returnvalue_4
    (for _index (range 1 (.Weight (Utilities|Struct|BreakS_Upgrade _array_element)))
      (Utilities|Array|Add (Variables|Default|GetUpgradeWeights) _array_index))))

(event EventTick
  (params (DeltaSeconds :type Float%20%28single-precision%29))
  (bind _returnvalue (Class|GameplayStatics|GetGlobalTimeDilation))
  (CallFunction|HandleDrift)
  (Transformation|SetActorLocation (Transformation|GetWorldLocation (Variables|Default|GetCube)) false false)
  (CallFunction|HandleCombo)
  (CallFunction|HandleCamera)
  (Utilities|FlowControl|Sequence
    (:then_0
      (CallFunction|Move (* (Input|EnhancedActionValues|GetIA_Move) (Math|Vector2D|MakeVector2D _returnvalue _returnvalue)))
      (CallFunction|HandleVolume)
      (CallFunction|HandleWheels))
    (:then_1
      ;[1 0.07031 0] Fail Timer
      (bind _output_get (Variables|Default|SetFailTimer (Math|Float|SelectFloat 15.0 (Math|Float|Max(Float) (- (Variables|Default|GetFailTimer) (Utilities|Time|GetWorldDeltaSeconds)) 0.0) (> (Math|Vector|VectorLength (Transformation|GetComponentVelocity (Variables|Default|GetCube))) 1e+02))))
      (if (== _output_get 0.0)
        (CallFunction|FailEvent)))))

(event Collision|EventHit
  (params (MyComp :type Primitive%20Component%20Object%20Reference) (Other :type Actor%20Object%20Reference) (OtherComp :type Primitive%20Component%20Object%20Reference) (bSelfMoved :type Boolean) (HitLocation :type Vector :default "0, 0, 0") (HitNormal :type Vector :default "0, 0, 0") (NormalImpulse :type Vector :default "0, 0, 0") (Hit :type Hit%20Result%20Structure%20%28by%20ref%29))
  ;[0.7344 0 1] Ram damage
  (Game|Damage|ApplyDamage Other (* (Math|Vector|VectorLength NormalImpulse) (CallFunction|GetProperty "NewEnumerator2")) (Game|GetPlayerController 0) self "/Script/Engine.DamageType"))

(event Input|KeyboardEvents|DebugKey1
  (params (Key :type Key%20Structure :default "None") (ActionValue :type Input%20Action%20Value%20Structure))
  (:Pressed
    (CallFunction|RequestUpgrade)))

(fn ConstructionScript)

(fn Move
  (params (Scale :type Vector%202D%20Structure))
  (Physics|AddForce (Variables|Default|GetCube) (* (Math|Vector|GetForwardVector (Variables|Default|GetCube)) (.x Scale) (CallFunction|GetProperty "NewEnumerator0") (- 1.0 (* (Input|EnhancedActionValues|GetIA_HandBrake) (Class|GameplayStatics|GetGlobalTimeDilation)))) "None" false)
  (Class|PrimitiveComponent|AddForceatLocation (Variables|Default|GetCube) (* (Math|Vector|GetRightVector (Variables|Default|GetCube)) (* (* (Math|Float|Sign(Float) (Math|Vector|DotProduct (Math|Vector|Normalize (Transformation|GetComponentVelocity (Variables|Default|GetCube))) (Math|Vector|GetForwardVector (Variables|Default|GetCube)))) (.y Scale) (Math|Vector|VectorLength (Transformation|GetComponentVelocity (Variables|Default|GetCube)))) (CallFunction|GetProperty "NewEnumerator1")) (+ (* (Input|EnhancedActionValues|GetIA_HandBrake) 2.0 (Class|GameplayStatics|GetGlobalTimeDilation)) 1.0)) (Transformation|GetWorldLocation (Variables|Default|GetSteeringLocation)) "None")
  (Audio|Parameter|SetFloatParameter (Variables|Default|GetMSC_Engine) "Throttle" (* (Math|Float|Absolute(Float) (.x Scale)) (* (Math|Vector|VectorLength (Transformation|GetComponentVelocity (Variables|Default|GetCube))) 0.0005)) :!class /Script/AudioExtensions.AudioParameterControllerInterface))

(fn ResetProperties
  (Utilities|Array|Resize (Variables|Default|GetProperties) (|GetNumEnumEntries))
  (CallFunction|SetProperty "NewEnumerator0" 1e+05)
  (CallFunction|SetProperty "NewEnumerator1" 3e+01)
  (CallFunction|SetProperty "NewEnumerator2" 0.07)
  (CallFunction|SetProperty "NewEnumerator3" 0.2)
  (CallFunction|SetProperty "NewEnumerator4" 1e+02))

(fn GetProperty
  (params (Property :type E_Properties%20Enum :default "NewEnumerator0"))
  (return (Utilities|Array|Get(acopy) (Variables|Default|GetProperties) (Math|Conversions|ToInteger(Byte) Property))))

(fn SetProperty
  (params (Property :type E_Properties%20Enum :default "NewEnumerator0") (Value :type Float%20%28double-precision%29))
  (Utilities|Array|SetArrayElem (Variables|Default|GetProperties) (Math|Conversions|ToInteger(Byte) Property) Value)
  (switch Utilities|FlowControl|Switch|SwitchonE_Properties Property
    (:NewEnumerator4
      (Class|PrimitiveComponent|SetMassOverrideinKg (Variables|Default|GetCube) "None" Value true))))

(fn GetSave
  (bind _returnvalue (SaveGame|DoesSaveGameExist "SaveData"))
  (if _returnvalue
    (bind _returnvalue_2 (SaveGame|LoadGamefromSlot "SaveData"))
    (bind _asbp_save_data (Utilities|Casting|CastToBP_SaveData _returnvalue_2))
    (return _asbp_save_data)
    (else
      (bind _returnvalue_3 (SaveGame|CreateSaveGameObject "/Game/Game/BP_SaveData.BP_SaveData_C"))
      (return _returnvalue_3))))

(fn HandleCamera
  (bind _returnvalue (Math|Float|MakeLiteralFloat 1e+02))
  (bind _springarm (Variables|Default|GetSpringArm))
  (bind _cube (Variables|Default|GetCube))
  (bind _returnvalue_2 (Transformation|GetComponentVelocity _cube))
  (bind _returnvalue_3 (- 0.0 _returnvalue))
  (bind _returnvalue_4 (Math|Vector|VectorLength _returnvalue_2))
  (bind _returnvalue_5 (* _returnvalue_4 0.5))
  (Variables|/Script/Engine.SpringArmComponent|SetTargetArmLength _springarm (+ _returnvalue_5 (* (Math|Float|Clamp(Float) (- _returnvalue_5 (Variables|/Script/Engine.SpringArmComponent|GetTargetArmLength _springarm)) _returnvalue_3 _returnvalue_3) (Utilities|Time|GetWorldDeltaSeconds)))))

(fn HandleVolume
  (Audio|SetSoundMixClassOverride "/Game/Sounds/SCM_Main.SCM_Main" "/Game/Sounds/SC_Main.SC_Main" (* (Math|Float|Clamp(Float) (Actor|GetGameTimeSinceCreation)) (Math|Float|Clamp(Float) (/ (Variables|Default|GetFailTimer) 5.0)) (Math|Float|Clamp(Float) (Class|GameplayStatics|GetGlobalTimeDilation) 0.01)) 1.0 0.0 true)
  (Audio|PushSoundMixModifier "/Game/Sounds/SCM_Main.SCM_Main"))

(fn HandleDrift
  (bind _value (CallFunction|GetProperty "NewEnumerator3"))
  (bind _cube (Variables|Default|GetCube))
  (bind _cube_2 (Variables|Default|GetCube))
  (bind _returnvalue (Transformation|GetComponentVelocity _cube))
  (bind _returnvalue_2 (Math|Vector|GetForwardVector _cube_2))
  (bind _returnvalue_3 (Math|Vector|VectorLength _returnvalue))
  (bind _returnvalue_4 (Math|Vector|Normalize _returnvalue))
  (bind _returnvalue_5 (Math|Vector|DotProduct _returnvalue_4 _returnvalue_2))
  (bind _returnvalue_6 (Math|Float|Absolute(Float) _returnvalue_5))
  (bind _returnvalue_7 (- 1.0 _returnvalue_6))
  (bind _returnvalue_8 (* _returnvalue_3 _returnvalue_7 _value))
  ;[0.3125 1 0] Smoke particles
  (Niagara|SetNiagaraVariable(Float) (Variables|Default|GetNiagara) "Rate" (* _returnvalue_8 (Math|Float|SelectFloat 1.0 0.0 (> _returnvalue_8 1.0))))
  (Audio|Parameter|SetFloatParameter (Variables|Default|GetMSC_Drift) "Amount" (Math|Float|Clamp(Float) (* _returnvalue_7 (Math|Vector|VectorLength (Transformation|GetComponentVelocity (Variables|Default|GetCube))) 0.01)) :!class /Script/AudioExtensions.AudioParameterControllerInterface))

(fn HandleWheels
  (bind _cube (Variables|Default|GetCube))
  (bind _fr (Variables|Default|GetFR))
  (bind _returnvalue (Transformation|GetComponentVelocity _cube))
  (bind _returnvalue_2 (Math|Vector|GetForwardVector _cube))
  (bind _returnvalue_3 (Math|Vector|DotProduct _returnvalue _returnvalue_2))
  (bind _returnvalue_4 (* (Math|Rotator|MakeRotator 0.0 _returnvalue_3 0.0) 0.023184))
  (Transformation|AddLocalRotation (Variables|Default|GetWheelFL) _returnvalue_4 false false)
  (Transformation|AddLocalRotation (Variables|Default|GetWheelRR) (* _returnvalue_4 -1.0) false false)
  (Transformation|SetRelativeRotation _fr (Math|Rotator|MakeRotator 0.0 0.0 (Math|Float|Lerp (* (.y (Input|EnhancedActionValues|GetIA_Move)) 3e+01 (Class|GameplayStatics|GetGlobalTimeDilation)) (.yaw (Variables|/Script/Engine.SceneComponent|GetRelativeRotation _fr)) 0.9)) false false))

(fn FailEvent
  (bind _returnvalue (Game|GetPlayerController 0))
  (bind _returnvalue_2 (CallFunction|GetSave))
  (Utilities|FlowControl|Sequence
    (:then_0
      (Variables|/Game/Game/BP_SaveData.BP_SaveData_C|SetHighScore _returnvalue_2 (Math|Integer|Max(Integer) (Variables|/Game/Game/BP_SaveData.BP_SaveData_C|GetHighScore _returnvalue_2) (Variables|Default|GetScore))))
    (:then_1
      (SaveGame|SaveGametoSlot _returnvalue_2 "SaveData"))
    (:then_2
      (Game|SetGamePaused true))
    (:then_3
      (bind _returnvalue_3 (UserInterface|CreateWidget "/Game/Player/Widgets/UI_FailScreen.UI_FailScreen_C"))
      (UserInterface|Viewport|AddtoViewport _returnvalue_3 0)
      (Input|SetInputModeUIOnly _returnvalue _returnvalue_3 "DoNotLock" true)
      (Variables|/Script/Engine.PlayerController|SetbShowMouseCursor _returnvalue true))))

(fn AddCombo
  (Variables|Default|SetScore (+ (Variables|Default|GetCurrentCombo) (Variables|Default|GetScore)))
  (Variables|Default|SetCurrentCombo 0)
  (Default|CallConfirmScore)
  (CallFunction|ResetComboScoreTimer))

(fn HandleCombo
  (bind _output_get (Variables|Default|SetComboTime (- (Variables|Default|GetComboTime) (Utilities|Time|GetWorldDeltaSeconds))))
  (if (and (<= _output_get 0.0) (> (Variables|Default|GetCurrentCombo) 0))
    (CallFunction|AddCombo)))

(fn GetRandomUpgrade
  (bind _output_get (LocalVariables|SetT (.OutItem (Utilities|Array|Random (Variables|Default|GetUpgradeWeights)))))
  (bind _returnvalue (Utilities|GetDataTableRow "/Game/Upgrades/DT_Upgrades.DT_Upgrades" (Utilities|Array|Get(acopy) (Variables|Default|GetUpgradeRowNames) _output_get))
    (:then
      (Utilities|FlowControl|Sequence
        (:then_0
          (if (not (.CanApplyTwice (Utilities|Struct|BreakS_Upgrade _returnvalue)))
            (Utilities|Array|RemoveItem (Variables|Default|GetUpgradeWeights) (LocalVariables|GetT))))
        (:then_1
          (return (.Class (Utilities|Struct|BreakS_Upgrade _returnvalue))))))))

(fn AddPhysicalUpgrade
  (params (Upgrade :type BP%20Physical%20Upgrade%20Class%20Reference))
  (if (Utilities|IsValidClass Upgrade)
    (bind _found (CallFunction|GetUpgrade Upgrade))
    (Utilities|IsValid _found
      (:Is%20Valid
        (Default|Upgrade _found))
      (:Is%20Not%20Valid
        (bind _returnvalue (Game|SpawnActorfromClass Upgrade (Math|Transform|MakeTransform "0, 0, 0" "0, 0, 0" "1.000000,1.000000,1.000000") "Undefined" 0 0))
        (Transformation|AttachComponentToComponent _returnvalue (Variables|Default|GetCube) "None" "KeepRelative" "KeepRelative" "KeepRelative" true)
        (Utilities|Array|Add (Variables|Default|GetAttachedActors) _returnvalue)))))

(fn GetUpgrade
  (params (Upgrade :type BP%20Physical%20Upgrade%20Class%20Reference))
  (for _array_element (Variables|Default|GetAttachedActors)
    (if (== (Utilities|GetClass _array_element) Upgrade)
      (return _array_element)))
  (return 0))