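; BP_Enemy is a base physics-driven vehicle enemy that chases the player using thrust and speed-scaled steering forces.
; Damage reduces Health, with mass scaling and a gated cooldown for blade and player hits, and updates hit audio, indicators and the health bar.
; Zero health or falling too low destroys it, triggering a Niagara mesh explosion and sound, awarding score and notifying its spawner.
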(event EventTick
  (params (DeltaSeconds :type Float%20%28single-precision%29))
  (bind _returnvalue (Game|Player|GetPlayerPawn 0))
  (bind _returnvalue_2 (Game|Player|GetPlayerPawn 0))
  (bind _cube (Variables|Default|GetCube))
  (bind _cube_2 (Variables|Default|GetCube))
  (bind _steeringforce (Variables|Default|GetSteeringForce))
  (bind _cube_3 (Variables|Default|GetCube))
  (bind _movingforce (Variables|Default|GetMovingForce))
  (bind _cube_4 (Variables|Default|GetCube))
  (bind _cube_5 (Variables|Default|GetCube))
  (bind _steerlocation (Variables|Default|GetSteerLocation))
  (bind _cube_6 (Variables|Default|GetCube))
  (bind _cube_7 (Variables|Default|GetCube))
  (bind _cube_8 (Variables|Default|GetCube))
  (bind _cube_9 (Variables|Default|GetCube))
  (bind _cube_10 (Variables|Default|GetCube))
  (bind _cube_11 (Variables|Default|GetCube))
  (bind _returnvalue_3 (Math|Vector|GetRightVector _cube_11))
  (bind _returnvalue_4 (Transformation|GetWorldLocation _steerlocation))
  (bind _returnvalue_5 (Transformation|GetComponentVelocity _cube))
  (bind _returnvalue_6 (Transformation|GetComponentVelocity _cube_10))
  (bind _returnvalue_7 (Math|Vector|GetForwardVector _cube_9))
  (bind _returnvalue_8 (Transformation|GetWorldLocation _cube_5))
  (bind _returnvalue_9 (Transformation|GetWorldLocation _cube_6))
  (bind _returnvalue_10 (Transformation|GetWorldRotation _cube_7))
  (bind _returnvalue_11 (Transformation|GetActorLocation _returnvalue))
  (bind _returnvalue_12 (Math|Vector|GetForwardVector _cube_3))
  (bind _returnvalue_13 (Transformation|GetWorldLocation _cube_8))
  (bind _returnvalue_14 (Transformation|GetActorLocation _returnvalue_2))
  (bind _returnvalue_15 (Math|Vector|GetForwardVector _cube_4))
  (bind _returnvalue_16 (Math|Vector|GetForwardVector _cube_2))
  (bind _returnvalue_17 (Math|Vector|VectorLength _returnvalue_6))
  (bind _returnvalue_18 (Math|Vector|Normalize _returnvalue_5))
  (bind _returnvalue_19 (- _returnvalue_14 _returnvalue_13))
  (bind _returnvalue_20 (- _returnvalue_11 _returnvalue_9))
  (bind _returnvalue_21 (Math|Vector|Normalize _returnvalue_20))
  (bind _returnvalue_22 (Math|Vector|DotProduct _returnvalue_18 _returnvalue_16))
  (bind _returnvalue_23 (Math|Vector|Normalize _returnvalue_19))
  (bind _returnvalue_24 (Math|Float|Sign(Float) _returnvalue_22))
  (bind _returnvalue_25 (Math|Vector|DotProduct _returnvalue_21 _returnvalue_15))
  (bind _returnvalue_26 (+ _returnvalue_7 _returnvalue_23))
  (bind _returnvalue_27 (Math|Vector|Normalize _returnvalue_26))
  (bind _returnvalue_28 (Math|Float|Sign(Float) _returnvalue_25))
  (bind _returnvalue_29 (Math|Rotator|MakeRotfromX _returnvalue_27))
  (bind _returnvalue_30 (* _returnvalue_12 _movingforce _returnvalue_28))
  (bind _returnvalue_31 (Math|Rotator|Delta(Rotator) _returnvalue_10 _returnvalue_29))
  (bind _returnvalue_32 (Math|Float|MapRangeClamped (.yaw _returnvalue_31) -3e+01 3e+01 -1.0 1.0))
  (bind _returnvalue_33 (* _returnvalue_24 _returnvalue_32 _returnvalue_17))
  (bind _returnvalue_34 (* _returnvalue_33 _steeringforce -1.0))
  (bind _returnvalue_35 (* _returnvalue_3 _returnvalue_34))
  (Class|PrimitiveComponent|AddForceatLocation (Variables|Default|GetCube) _returnvalue_35 (Transformation|GetWorldLocation (Variables|Default|GetSteerLocation)) "None")
  ;[0.1484 1 0] Engine thrust
  (Physics|AddForce (Variables|Default|GetCube) _returnvalue_30 "None" false)
  (Utilities|FlowControl|Sequence
    (:then_0
      (if (< (.z (Transformation|GetWorldLocation (Variables|Default|GetCube))) -1e+04)
        (Actor|DestroyActor)))
    (:then_1
      (if (Variables|Default|GetDebug)
        (Rendering|Debug|DrawDebugArrow _returnvalue_8 (+ _returnvalue_8 (* _returnvalue_30 0.1)) 1e+02 "(R=1.000000,G=0.000000,B=0.005617,A=1.000000)" 0.0 1e+01)
        (Rendering|Debug|DrawDebugArrow _returnvalue_4 (+ _returnvalue_4 (* _returnvalue_35 0.3)) 1e+02 "(R=0.000000,G=0.023826,B=1.000000,A=1.000000)" 0.0 1e+01)))))

(event Game|Damage|EventAnyDamage
  (params (Damage :type Float%20%28single-precision%29) (DamageType :type Damage%20Type%20Object%20Reference) (InstigatedBy :type Controller%20Object%20Reference) (DamageCauser :type Actor%20Object%20Reference))
  (bind _returnvalue (Utilities|GetClass DamageCauser))
  (bind _set (Utilities|Set|MakeSet "/Game/Upgrades/Upgrades/Blades/BP_Blades.BP_Blades_C" "/Game/Player/BP_PlayerCharacter.BP_PlayerCharacter_C"))
  (bind _mass (Variables|Default|GetMass))
  (bind _msc_hit (Variables|Default|GetMSC_Hit))
  (bind _returnvalue_2 (Utilities|Set|Contains _set _returnvalue))
  (bind _returnvalue_3 (Math|Float|SelectFloat _mass 1.0 _returnvalue_2))
  (bind _returnvalue_4 (/ Damage _returnvalue_3))
  (if _returnvalue_2
    ;[0.05469 1 0] Damage
    (Utilities|FlowControl|Gate false :!label _label
      (:Exit
        _)))
  (Utilities|FlowControl|Sequence
    (:then_0
      (Audio|Parameter|SetFloatParameter _msc_hit "Magnitude" (* _returnvalue_4 0.01) :!class /Script/AudioExtensions.AudioParameterControllerInterface)
      (Audio|Components|Audio|Play _msc_hit 0.0))
    (:then_1
      (Game|SpawnActorfromClass "/Game/Enemies/Base/BP_DamageIndicator.BP_DamageIndicator_C" (Transformation|GetWorldTransform (Variables|Default|GetCube)) "AlwaysSpawn" 0 _returnvalue_4 (.Health (Utilities|GetClassDefaults (Utilities|GetClass self))) 0))
    (:then_2
      (bind _output_get (Variables|Default|SetHealth (- (Variables|Default|GetHealth) _returnvalue_4)))
      (if (<= _output_get 0.0)
        (Actor|DestroyActor)))
    (:then_3
      (Utilities|FlowControl|Delay 0.5)
      (goto _label Open))
    (:then_4
      (if _returnvalue_2
        (goto _label Close)))
    (:then_5
      (Default|Update (Variables|Default|GetUI)))))

(event EventDestroyed
  (bind _cube (Variables|Default|GetCube))
  (bind _returnvalue (Transformation|GetWorldTransform _cube))
  ;[0 1 0.8594] Explosion
  (bind _returnvalue_2 (Niagara|SpawnSystematLocation "/Game/Enemies/Base/ExplosionEffect/SN_ExplodingVehicle.SN_ExplodingVehicle" (.location _returnvalue) (.rotation _returnvalue) (.scale _returnvalue)))
  (Class|NiagaraComponent|SetVariableStaticMesh _returnvalue_2 "Mesh" (Variables|/Script/Engine.StaticMeshComponent|GetStaticMesh (Variables|Default|GetCube)))
  (bind _asbp_player_character (Utilities|Casting|CastToBP_PlayerCharacter (Game|Player|GetPlayerPawn 0)))
  (Default|AddScoreEvent _asbp_player_character (Variables|Default|GetScoreOnKill) "NewEnumerator0")
  (Audio|PlaySoundatLocation "/Game/Sounds/Cues/MSC_Explosion.MSC_Explosion" (Transformation|GetWorldLocation (Variables|Default|GetCube)) "0, 0, 0" (Math|Random|RandomFloatinRange 0.8 1.2) (Math|Random|RandomFloatinRange 0.8 1.2) 0.0 0 0 0 0)
  (Default|OnKill (Variables|Default|GetSpawner)))

(event EventBeginPlay
  ;[0.7813 0 1] Begin play
  (bind _asui_health_bar (Utilities|Casting|CastToUI_HealthBar (UserInterface|GetWidget (Variables|Default|GetWidget))))
  (bind _output_get (Variables|Default|SetUI _asui_health_bar))
  (Variables|/Game/Enemies/Base/UI_HealthBar.UI_HealthBar_C|SetEnemy _output_get self)
  (Class|PrimitiveComponent|SetMassOverrideinKg (Variables|Default|GetCube) "None" (Variables|Default|GetMass) true))

(fn ConstructionScript)