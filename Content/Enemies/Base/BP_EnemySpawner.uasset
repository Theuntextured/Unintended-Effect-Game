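; Round-based enemy spawner that spawns weighted random enemies around the player and shows a round indicator widget each round.
; Each round, a looping timer spreads a growing, power-curve spawn count over the deploy time, using line traces within a box to place enemies facing the player.
; Kills reaching zero remaining advance the round, alongside a restarted round-increase timer.
; The construction script builds the weighted pool and draws the box, both only under Debug.
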(event Custom|RequestSpawn
  (if (not (== (Variables|Default|GetEnemiesSpawned) (CallFunction|GetSpawnCountinRound)))
    (CallFunction|SpawnEnemy)))

(event Custom|IncrementRound
  (Utilities|Time|ClearandInvalidateTimerbyHandle (Variables|Default|GetRoundIncreaseTimer))
  (Variables|Default|SetEnemiesSpawned 0)
  (Utilities|Time|ClearandInvalidateTimerbyHandle (Variables|Default|GetSpawnTimer))
  (Math|Integer|IncrementInt (Variables|Default|GetRound)
    (:%20%20
      (bind _returnvalue (Utilities|Time|SetTimerbyEvent (delegate Custom|RequestSpawn) (/ (Variables|Default|GetRoundDeployTime) (CallFunction|GetSpawnCountinRound)) true))
      (Variables|Default|SetSpawnTimer _returnvalue)
      (bind _returnvalue_2 (UserInterface|CreateWidget "/Game/Enemies/Base/UI_RoundIndicator.UI_RoundIndicator_C" 0 (Variables|Default|GetRound)))
      (UserInterface|Viewport|AddtoViewport _returnvalue_2 0)
      (bind _returnvalue_3 (Utilities|Time|SetTimerbyEvent (EventDispatchers|CreateEvent :!event Custom|IncrementRound) 6e+01))
      (Variables|Default|SetRoundIncreaseTimer _returnvalue_3))))

(event Custom|OnKill
  (bind _enemiesremaining (Variables|Default|GetEnemiesRemaining))
  (Math|Integer|DecrementInt _enemiesremaining
    (:%20%20
      (if (== _enemiesremaining 0)
        (CallFunction|IncrementRound)))))

(event EventBeginPlay
  (CallFunction|IncrementRound))

(fn ConstructionScript
  (bind _enemyweights (Variables|Default|GetEnemyWeights))
  (if (Variables|Default|GetDebug)
    (Rendering|Debug|FlushPersistentDebugLines)
    (Rendering|Debug|DrawDebugBox (Transformation|GetActorLocation) (Variables|Default|GetBoxExtent) "(R=0.000000,G=0.148525,B=1.000000,A=1.000000)" "0, 0, 0" 5.0 5.0)
    (bind _keys (Utilities|Map|Keys _enemyweights))
    (bind _values (Utilities|Map|Values _enemyweights))
    (for (_array_element _array_index) _keys
      (for _index (range 1 (Utilities|Array|Get(acopy) _values _array_index))
        (Utilities|Array|Add (Variables|Default|GetWeightedEnemies) _array_element)))))

(fn SpawnEnemy
  (bind _returnvalue (Game|Player|GetPlayerPawn 0))
  (bind _boxextent (Variables|Default|GetBoxExtent))
  (bind _returnvalue_2 (Transformation|GetActorLocation _returnvalue))
  (bind _z (Class|KismetMathLibrary|BreakVector3f _boxextent))
  (bind _returnvalue_3 (Math|Random|RandomPointinBoundingBox _returnvalue_2 _boxextent))
  (bind _z_2 (Class|KismetMathLibrary|BreakVector3f _returnvalue_2))
  (bind (_outhit _returnvalue_4) (Collision|LineTraceByChannel (Math|Vector|MakeVector (.x _returnvalue_3) (.y _returnvalue_3) (+ _z_2 _z)) (Math|Vector|MakeVector (.x _returnvalue_3) (.y _returnvalue_3) (- _z_2 _z)) "TraceTypeQuery1" false 0 "None"))
  (if _returnvalue_4
    (Game|SpawnActorfromClass (CallFunction|GetEnemySpawnType) (Math|Transform|MakeTransform (.Location (Collision|BreakHitResult _outhit)) (Math|Conversions|RotationFromXVector (- (Transformation|GetActorLocation (Game|Player|GetPlayerPawn 0)) (.Location (Collision|BreakHitResult _outhit)))) "1.000000,1.000000,1.000000") "AlwaysSpawn" 0 self 0)
    (Math|Integer|IncrementInt (Variables|Default|GetEnemiesSpawned)
      (:%20%20
        (Math|Integer|IncrementInt (Variables|Default|GetEnemiesRemaining))))))

(fn GetEnemySpawnType
  (return (.OutItem (Utilities|Array|Random (Variables|Default|GetWeightedEnemies)))))

(fn GetSpawnCountinRound
  (return (Math|Float|Round (* (Math|Float|Power (Math|Conversions|ToFloat(Integer) (Variables|Default|GetRound)) 1.5) 3.0))))