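; BP_DamageIndicator is a short-lived actor that displays a damage number through a widget component.
; On BeginPlay it destroys itself immediately when Damage is below 1.
; Otherwise it builds its UI_DamageIndicator widget from Damage and MaxHP, then destroys itself after a brief delay.
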(event EventBeginPlay
  (if (< (Variables|Default|GetDamage) 1.0)
    (Actor|DestroyActor)
    (else
      (bind _asui_damage_indicator (Utilities|Casting|CastToUI_DamageIndicator (UserInterface|GetWidget (Variables|Default|GetWidget))))
      (Default|Build _asui_damage_indicator (Variables|Default|GetDamage) (Variables|Default|GetMaxHP))
      (Utilities|FlowControl|Delay 1.5)
      (Actor|DestroyActor))))

(fn ConstructionScript)