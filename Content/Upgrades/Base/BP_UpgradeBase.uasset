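; BP_UpgradeBase is the base upgrade Blueprint, applying a set of stat changes and a physical upgrade to a character.
; ApplyUpgrade loops over the Upgrades array, setting each character property to the entry's value when Override is set, otherwise multiplying the current value by it.
; It then passes PhysicalUpgrade to the character's AddPhysicalUpgrade and calls CallUpgraded on the character.
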(fn ApplyUpgrade
  (bind _character (Variables|Default|GetCharacter))
  (Utilities|FlowControl|Sequence
    (:then_0
      (for _array_element (Variables|Default|GetUpgrades)
        (Default|SetProperty _character (.Property (Utilities|Struct|BreakS_StatUpgrade _array_element)) (Math|Float|SelectFloat (.Value (Utilities|Struct|BreakS_StatUpgrade _array_element)) (* (Default|GetProperty _character (.Property (Utilities|Struct|BreakS_StatUpgrade _array_element))) (.Value (Utilities|Struct|BreakS_StatUpgrade _array_element))) (.Override (Utilities|Struct|BreakS_StatUpgrade _array_element))))))
    (:then_1
      (Default|AddPhysicalUpgrade (Variables|Default|GetCharacter) (Variables|Default|GetPhysicalUpgrade)))
    (:then_2
      (Default|CallUpgraded (Variables|Default|GetCharacter)))))