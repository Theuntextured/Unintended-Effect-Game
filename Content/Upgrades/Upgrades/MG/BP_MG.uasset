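; BP_MG is a machine gun upgrade that fires hitscan shots for the player.
; A looping timer is set from FireRate, and RefreshProperties rebuilds it and updates the Niagara particle count.
; Shoot restarts both effects, plays a pitch-varied gunshot, line-traces forward to apply damage, and pushes the player's Cube backward as recoil.
; Upgrade trades lower per-shot damage for higher fire rate and more particles.
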(event EventBeginPlay
  (bind _asbp_player_character (Utilities|Casting|CastToBP_PlayerCharacter (Game|Player|GetPlayerPawn 0)))
  (Variables|Default|SetAs%20BP%20Player%20Character _asbp_player_character)
  (CallFunction|RefreshProperties)
  (CallFunction|Shoot))

(fn ConstructionScript
  (|CallParentFunction))

(fn RefreshProperties
  (Niagara|SetNiagaraVariable(Float) (Variables|Default|GetNiagara) "ParticleCount" (Variables|Default|GetParticleAmount))
  (Utilities|Time|ClearandInvalidateTimerbyHandle (Variables|Default|GetShootTimer))
  (bind _returnvalue (Utilities|Time|SetTimerbyEvent (EventDispatchers|CreateEvent :!event Shoot) (/ 6e+01 (Variables|Default|GetFireRate)) true))
  (Variables|Default|SetShootTimer _returnvalue))

(fn Upgrade
  (Variables|Default|SetDamage (* (Variables|Default|GetDamage) 0.85))
  (Variables|Default|SetFireRate (* (Variables|Default|GetFireRate) 1.2))
  (Variables|Default|SetParticleAmount (* (Variables|Default|GetParticleAmount) 1.5))
  (CallFunction|RefreshProperties))

(fn Shoot
  (bind _as_bp_player_character (Variables|Default|GetAs%20BP%20Player%20Character))
  (bind _scene (Variables|Default|GetScene))
  (bind _returnvalue (Transformation|GetWorldLocation _scene))
  (bind _cube (Variables|/Game/Player/BP_PlayerCharacter.BP_PlayerCharacter_C|GetCube _as_bp_player_character))
  (Utilities|FlowControl|Sequence
    (:then_0
      (Niagara|ResetSystem (Variables|Default|GetNiagara1))
      (Audio|PlaySoundatLocation "/Game/Sounds/Cues/SC_Gunshot.SC_Gunshot" (Transformation|GetWorldLocation (Variables|Default|GetNiagara)) "0, 0, 0" 0.35 (Math|Random|RandomFloatinRange 0.9 1.1) 0.0 0 0 0 0)
      (bind (_outhit _returnvalue_2) (Collision|LineTraceByChannel _returnvalue (+ (* (Math|Vector|GetForwardVector _scene) 5e+03) _returnvalue) "TraceTypeQuery1" false (Utilities|Array|MakeArray (Game|Player|GetPlayerPawn 0)) "None"))
      (if _returnvalue_2
        (Game|Damage|ApplyDamage (.hitactor _outhit) (Variables|Default|GetDamage) (Game|GetPlayerController 0) self "/Script/Engine.DamageType")))
    (:then_1
      (Physics|AddImpulse _cube (* (Math|Vector|NegateVector (Math|Vector|GetForwardVector _cube)) (Variables|Default|GetRecoil)) "None" false))))