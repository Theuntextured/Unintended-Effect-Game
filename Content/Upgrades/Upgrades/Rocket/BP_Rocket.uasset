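; BP_Rocket is an upgradeable rocket booster that pushes the player character's Cube along its forward vector.
; Tick applies a constant passive thrust, adds full Power while active, and drains or recharges a clamped Charge.
; Activation requires full charge and enables the Niagara and MSCRocket effects, while empty charge deactivates it.
; Upgrade raises power and passive thrust but lengthens recharge time, and BeginPlay creates the rocket's UI widget.
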(event Custom|Activate
  (if (== (Variables|Default|GetCharge) 1.0)
    (Components|Activation|SetActive (Variables|Default|GetNS_Rocket) true false)
    (Variables|Default|SetisActive true)
    (Components|Activation|SetActive (Variables|Default|GetMSC_Rocket) true false)))

(event Custom|Deactivate
  (Components|Activation|SetActive (Variables|Default|GetNS_Rocket) false false)
  (Variables|Default|SetisActive false)
  (Components|Activation|SetActive (Variables|Default|GetMSC_Rocket) false false))

(event EventBeginPlay
  (CallFunction|Deactivate)
  (bind _asbp_player_character (Utilities|Casting|CastToBP_PlayerCharacter (Game|Player|GetPlayerPawn 0)))
  (Variables|Default|SetAs%20BP%20Player%20Character _asbp_player_character)
  (bind _returnvalue (UserInterface|CreateWidget "/Game/Upgrades/Upgrades/Rocket/UI_RocketUI.UI_RocketUI_C" 0 self))
  (UserInterface|Viewport|AddtoViewport _returnvalue -1))

(event EventTick
  (params (DeltaSeconds :type Float%20%28single-precision%29))
  (bind _as_bp_player_character (Variables|Default|GetAs%20BP%20Player%20Character))
  (bind _power (Variables|Default|GetPower))
  (bind _passivepowermult (Variables|Default|GetPassivePowerMult))
  (bind _returnvalue (* _passivepowermult _power))
  (bind _cube (Variables|/Game/Player/BP_PlayerCharacter.BP_PlayerCharacter_C|GetCube _as_bp_player_character))
  (Physics|AddForce _cube (* (Math|Vector|GetForwardVector _cube) (Math|Float|SelectFloat (+ _power _returnvalue) _returnvalue (Variables|Default|GetisActive))) "None" false)
  (bind _output_get (Variables|Default|SetCharge (Math|Float|Clamp(Float) (+ (Variables|Default|GetCharge) (* (Math|Float|SelectFloat -1.0 (/ 1.0 (Variables|Default|GetChargeTime)) (Variables|Default|GetisActive)) (Utilities|Time|GetWorldDeltaSeconds))))))
  (if (== _output_get 0.0)
    (CallFunction|Deactivate)))

(fn ConstructionScript
  (|CallParentFunction))

(fn Upgrade
  (Variables|Default|SetPower (* (Variables|Default|GetPower) 1.15))
  (Variables|Default|SetChargeTime (* (Variables|Default|GetChargeTime) 1.2))
  (Variables|Default|SetPassivePowerMult (+ (Variables|Default|GetPassivePowerMult) 0.05)))