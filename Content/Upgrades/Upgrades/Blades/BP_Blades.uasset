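; BP_Blades is an upgrade with left and right spinning blades that damage enemies.
; Each tick both blades spin up toward a max RPM, which drives rotation and an audio parameter.
; Overlapping BP_Enemy actors take per-frame damage scaled by that side's RPM, which depletes it, with an extra drop if the enemy becomes invalid.
; BeginPlay adds a blades UI widget, and Upgrade rescales the spin, damage and depletion stats.
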(event EventTick
  (params (DeltaSeconds :type Float%20%28single-precision%29))
  (bind _returnvalue (Game|GetPlayerController 0))
  (bind _returnvalue_2 (Math|Float|MakeLiteralFloat 0.2))
  (bind _self self)
  (Utilities|FlowControl|Sequence
    (:then_0
      (Variables|Default|SetRPML (Math|Float|Clamp(Float) (+ (Variables|Default|GetRPML) (* (Utilities|Time|GetWorldDeltaSeconds) (Variables|Default|GetSpinPower))) 0.0 (Variables|Default|GetMaxRPM)))
      (Variables|Default|SetRPMR (Math|Float|Clamp(Float) (+ (Variables|Default|GetRPMR) (* (Utilities|Time|GetWorldDeltaSeconds) (Variables|Default|GetSpinPower))) 0.0 (Variables|Default|GetMaxRPM)))
      (Transformation|AddLocalRotation (Variables|Default|GetBladeL) (Math|Rotator|MakeRotator 0.0 0.0 (* (Variables|Default|GetRPML) _returnvalue_2)) false false)
      (Transformation|AddLocalRotation (Variables|Default|GetBladeR) (Math|Rotator|MakeRotator 0.0 0.0 (* (Variables|Default|GetRPMR) _returnvalue_2)) false false)
      (Audio|Parameter|SetFloatParameter (Variables|Default|GetMSC_BladeL) "RPM" (Variables|Default|GetRPML) :!class /Script/AudioExtensions.AudioParameterControllerInterface)
      (Audio|Parameter|SetFloatParameter (Variables|Default|GetMSC_BladeR) "RPM" (Variables|Default|GetRPMR) :!class /Script/AudioExtensions.AudioParameterControllerInterface))
    (:then_1
      (for _array_element (Collision|GetOverlappingActors (Variables|Default|GetCollisionR) "/Game/Enemies/Base/BP_Enemy.BP_Enemy_C" :!class /Script/Engine.PrimitiveComponent)
        (bind _output_get (Variables|Default|SetT _array_element))
        (Game|Damage|ApplyDamage _output_get (* (Variables|Default|GetRPMR) (Variables|Default|GetBladeDamageMultiplier)) _returnvalue _self "/Script/Engine.DamageType")
        (Variables|Default|SetRPMR (* (Math|Float|Power (Variables|Default|GetRPMDepletionRate) (Utilities|Time|GetWorldDeltaSeconds)) (Variables|Default|GetRPMR)))
        (Variables|Default|GetT
          (:then)
          (:else
            (Variables|Default|SetRPMR (* (Variables|Default|GetRPMR) (Variables|Default|GetRPMDepletionRate))))))
      (for _array_element_2 (Collision|GetOverlappingActors (Variables|Default|GetCollisionL) "/Game/Enemies/Base/BP_Enemy.BP_Enemy_C" :!class /Script/Engine.PrimitiveComponent)
        (bind _output_get_2 (Variables|Default|SetT _array_element_2))
        (Game|Damage|ApplyDamage _output_get_2 (* (Variables|Default|GetRPML) (Variables|Default|GetBladeDamageMultiplier)) _returnvalue _self "/Script/Engine.DamageType")
        (Variables|Default|SetRPML (* (Math|Float|Power (Variables|Default|GetRPMDepletionRate) (Utilities|Time|GetWorldDeltaSeconds)) (Variables|Default|GetRPML)))
        (Variables|Default|GetT
          (:then)
          (:else
            (Variables|Default|SetRPML (* (Variables|Default|GetRPML) (Variables|Default|GetRPMDepletionRate)))))))))

(event EventBeginPlay
  (bind _returnvalue (UserInterface|CreateWidget "/Game/Upgrades/Upgrades/Blades/UI_BladesUI.UI_BladesUI_C" 0 self))
  (UserInterface|Viewport|AddtoViewport _returnvalue -1))

(fn ConstructionScript
  (|CallParentFunction))

(fn Upgrade
  (Variables|Default|SetMaxRPM (* (Variables|Default|GetMaxRPM) 1.2))
  (Variables|Default|SetSpinPower (* (Variables|Default|GetSpinPower) 1.2))
  (Variables|Default|SetBladeDamageMultiplier (* (Variables|Default|GetBladeDamageMultiplier) 1.2))
  (Variables|Default|SetRPMDepletionRate (/ (Variables|Default|GetRPMDepletionRate) 1.2)))