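; Main menu pawn that shows the title UI and starts the game on any key press.
; On BeginPlay it creates the UI_MainMenu widget, plays its Enter animation, then opens an input gate after a short delay.
; The first key press through the gate plays that animation in reverse and, when it finishes, calls StartGame on BP_GameInstance.
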(event EventBeginPlay
  (bind _returnvalue (UserInterface|CreateWidget "/Game/MainMenu/UI_MainMenu.UI_MainMenu_C"))
  (UserInterface|Viewport|AddtoViewport _returnvalue 0)
  (bind _output_get (Variables|Default|SetUI _returnvalue))
  (UserInterface|Animation|PlayAnimation _output_get (Variables|/Game/MainMenu/UI_MainMenu.UI_MainMenu_C|GetEnter _output_get) 0.0 1 "Forward" 1.0 false)
  (Utilities|FlowControl|Delay 2.0)
  (Utilities|FlowControl|Gate true) ; enters at Open
)

(event Input|KeyboardEvents|AnyKey
  (params (Key :type Key%20Structure :default "None"))
  (bind _ui (Variables|Default|GetUI))
  (:Pressed
    (Utilities|FlowControl|Gate true
      (:Exit
        (Utilities|FlowControl|DoOnce false
          (:Completed
            (Components|Animation|PlayAnimation _ui (Variables|/Game/MainMenu/UI_MainMenu.UI_MainMenu_C|GetEnter _ui) 0.0 1 "Reverse"
              (:Finished
                (bind _asbp_game_instance (Utilities|Casting|CastToBP_GameInstance (Game|GetGameInstance)))
                (Default|StartGame _asbp_game_instance)))))))))

(fn ConstructionScript)